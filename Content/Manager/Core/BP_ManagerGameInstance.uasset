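; Game instance for a management simulation that holds the current simulation variant data, including its employees and user stories.
; Functions replace the whole variant, look up an employee or user story by ID, or overwrite the fields of the matching array entry in place.
; UpdateVarData and OnDataReceived are empty, and the HUD-based request for fresh variant data is left unconnected.
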(fn UpdateSimulationVariantData
  (params (VariantData :type Sim%20Variant%20Data%20Structure))
  (Variables|Default|SetCurrentSimulationVariantData VariantData))

(fn FindUserStory
  (params (Index :type Integer))
  (bind _array_element (Utilities|Array|ForEachLoopwithBreak (.UserStories (Utilities|Struct|BreakSimVariantData (Variables|Default|GetCurrentSimulationVariantData))))
    (:LoopBody
      (if (== (.ID (Utilities|Struct|BreakUSData _array_element)) Index)
        (return _array_element)))))

(fn UpdateEmployees
  (params (Employee :type Employee%20Data%20Structure) (ID :type Integer))
  (bind (_id _name _description _thumbnail _maxhours _maxtasks _skill _proficiency _buffs _debuffs) (Utilities|Struct|BreakEmployeeData Employee))
  (bind (_array_element _array_index) (Utilities|Array|ForEachLoopwithBreak (Utilities|Struct|BreakSimVariantData (Variables|Default|GetCurrentSimulationVariantData)) :!label _label)
    (:LoopBody
      (if (== (Utilities|Struct|BreakEmployeeData _array_element) ID)
        (goto _label Break)))
    (:Completed
      (Utilities|Struct|SetmembersinEmployeeData (Utilities|Array|Get(acopy) (Utilities|Struct|BreakSimVariantData (Variables|Default|GetCurrentSimulationVariantData)) _array_index) _name _description _maxhours _maxtasks _skill _proficiency _buffs _debuffs))))

(fn UpdateUserStories
  (params (UserStory :type US%20Data%20Structure) (ID :type Integer))
  (bind (_array_element _array_index) (Utilities|Array|ForEachLoopwithBreak (Utilities|Struct|BreakSimVariantData (Variables|Default|GetCurrentSimulationVariantData)) :!label _label)
    (:LoopBody
      (if (== (Utilities|Struct|BreakUSData _array_element) ID)
        (goto _label Break)))
    (:Completed
      (Utilities|Struct|SetmembersinUSData (Utilities|Array|Get(acopy) (Utilities|Struct|BreakSimVariantData (Variables|Default|GetCurrentSimulationVariantData)) _array_index) (.description UserStory) (.complexity UserStory) (.hours UserStory) (.dobefore UserStory) (.childus UserStory) (.parentus UserStory) (.proficiencies UserStory)))))

(fn FindEmployee
  (params (ID :type Integer))
  (for _array_element (.Employees (Utilities|Struct|BreakSimVariantData (Variables|Default|GetCurrentSimulationVariantData)))
    (if (== (.ID (Utilities|Struct|BreakEmployeeData _array_element)) ID)
      (return _array_element))))

(fn UpdateVarData)

(fn OnDataReceived
  (params (Success :type Boolean) (SimVariantData :type Sim%20Variant%20Data%20Structure%20%28by%20ref%29)))